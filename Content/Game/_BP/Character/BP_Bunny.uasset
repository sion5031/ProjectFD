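; BP_Bunny is a bunny character that starts with random equipment items in its inventory.
; On BeginPlay, only with authority, it waits briefly, then adds one random pick from EquipmentItems to its InventoryComponent per count of ItemNum.
; The construction script sets Mesh as leader pose for BodyMesh, so the body follows the main skeleton's animation.
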(event EventBeginPlay
  (if (Ability|HasAuthority)
    (Utilities|FlowControl|Delay 0.2)
    (while (> (Variables|Default|GetItem%20Num) 0)
      (Class|InventoryComponent|AddItem (Variables|Default|GetInventoryComponent) (.OutItem (Utilities|Array|Random (Variables|Default|GetEquipment%20Items))) 1)
      (Math|Integer|DecrementInt (Variables|Default|GetItem%20Num)))))

(event Collision|EventActorBeginOverlap
  (params (OtherActor :type Actor%20Object%20Reference)))

(event EventTick
  (params (DeltaSeconds :type Float%20%28single-precision%29)))

(fn ConstructionScript
  (Components|SkinnedMesh|SetLeaderPoseComponent (Variables|Default|GetBodyMesh) (Variables|Character|GetMesh) false false))