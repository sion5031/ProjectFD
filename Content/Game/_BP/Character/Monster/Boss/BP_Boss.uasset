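; Boss monster Blueprint that shows health and shield bars through a widget component on non-authority clients.
; On BeginPlay, the authority destroys the widget component, so the bars exist only where the actor lacks authority.
; Each Tick without authority casts the widget to TESTWIDGET and sets its HP and Shield to current-over-max ratios read from EnemyAttributeSet.
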(event EventBeginPlay
  (if (Ability|HasAuthority)
    (Components|DestroyComponent (Variables|Default|GetWidget))))

(event Collision|EventActorBeginOverlap
  (params (OtherActor :type Actor%20Object%20Reference)))

(event EventTick
  (params (DeltaSeconds :type Float%20%28single-precision%29))
  (bind _enemyattributeset (Variables|Default|GetEnemyAttributeSet))
  (if (not (Ability|HasAuthority))
    (bind _astestwidget (Utilities|Casting|CastToTESTWIDGET (UserInterface|GetUserWidgetObject (Variables|Default|GetWidget))))
    (Variables|/Game/Game/_BP/Character/Monster/Boss/TESTWIDGET.TESTWIDGET_C|SetHP _astestwidget (/ (.CurrentValue (Utilities|Struct|BreakGameplayAttributeData (Variables|/Script/ProjectFD.FDAttributeSet|GetHealth _enemyattributeset))) (.CurrentValue (Utilities|Struct|BreakGameplayAttributeData (Variables|/Script/ProjectFD.FDAttributeSet|GetMaxHealth _enemyattributeset)))))
    (Variables|/Game/Game/_BP/Character/Monster/Boss/TESTWIDGET.TESTWIDGET_C|SetShield _astestwidget (/ (.CurrentValue (Utilities|Struct|BreakGameplayAttributeData (Variables|/Script/ProjectFD.FDAttributeSet|GetShield _enemyattributeset))) (.CurrentValue (Utilities|Struct|BreakGameplayAttributeData (Variables|/Script/ProjectFD.FDAttributeSet|GetMaxShield _enemyattributeset)))))))

(fn ConstructionScript)