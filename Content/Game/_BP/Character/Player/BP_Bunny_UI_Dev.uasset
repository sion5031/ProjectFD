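; BP_Bunny_UI_Dev is a development variant of the Bunny player character with debug hotkeys that fill the inventory, apparently for UI work.
; T adds every entry in EquipmentItems to the InventoryComponent, and Y adds the first CheatWeapon with its own acquisition info.
; An unconnected authority-only chain would grant random equipment and modules after a short delay.
; The construction script makes BodyMesh follow the main Mesh's pose.
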(event EventBeginPlay)

(event Input|KeyboardEvents|T
  (params (Key :type Key%20Structure :default "None"))
  (:Pressed
    (for _array_element (Variables|Default|GetEquipment%20Items)
      (Class|InventoryComponent|AddItem (Variables|Default|GetInventoryComponent) _array_element (Variables|Default|GetAcquisition%20Info) 1))))

(event Input|KeyboardEvents|Y
  (params (Key :type Key%20Structure :default "None"))
  (:Pressed
    (Class|InventoryComponent|AddItem (Variables|Default|GetInventoryComponent) (Utilities|Array|Get(acopy) (Variables|Default|GetCheatWeapon)) (Variables|Default|GetCheatAcquisitionInfo) 1)))

(fn ConstructionScript
  (Components|SkinnedMesh|SetLeaderPoseComponent (Variables|Default|GetBodyMesh) (Variables|Character|GetMesh) false false))