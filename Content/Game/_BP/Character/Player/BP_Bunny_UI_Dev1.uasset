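; Development variant of the Bunny player character, named for UI work, that fills its inventory with random items.
; On BeginPlay the authority waits briefly, then loops adding random equipment and module items to InventoryComponent; the module loop decrements ItemNum instead of ModuleNum, so its condition never changes.
; The construction script makes BodyMesh follow the main Mesh pose.
; Weapon-fire toggle and hand-socket alignment nodes are left unconnected.
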(event EventBeginPlay
  (if (Ability|HasAuthority)
    (Utilities|FlowControl|Delay 0.2)
    (while (> (Variables|Default|GetItem%20Num) 0)
      (Class|InventoryComponent|AddItem (Variables|Default|GetInventoryComponent) (.OutItem (Utilities|Array|Random (Variables|Default|GetEquipment%20Items))) (Variables|Default|GetAcquisition%20Info) 1)
      (Math|Integer|DecrementInt (Variables|Default|GetItem%20Num)))
    (while (> (Variables|Default|GetModuleNum) 0)
      (Class|InventoryComponent|AddItem (Variables|Default|GetInventoryComponent) (.OutItem (Utilities|Array|Random (Variables|Default|GetModuleItems))) (Variables|Default|GetAcquisition%20Info) 1)
      (Math|Integer|DecrementInt (Variables|Default|GetItem%20Num)))))

(event Input|MouseEvents|ThumbMouseButton2
  (params (Key :type Key%20Structure)))

(fn ConstructionScript
  (Components|SkinnedMesh|SetLeaderPoseComponent (Variables|Default|GetBodyMesh) (Variables|Character|GetMesh) false false))